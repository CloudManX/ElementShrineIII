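; BP_ForceApplier pulses the "ApplyForce?" flag in the NPC_FxManager Niagara Parameter Collection when T is pressed.
; The key press records the current frame number, and Tick sets the flag true only while the frame count matches it.
; On every other frame Tick resets the flag to false, giving a single-frame trigger.
; Both branches print a short-lived debug string showing the current state.
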(event `Key|T`
  (params (Key :type "Key Structure"))
  (:`Pressed`
    (set `self.CurrentFrame` (`KismetSystemLibrary.GetFrameCount`))))

(event `self.ReceiveTick`
  (params (DeltaSeconds :type "Float (single-precision)"))
  (if (== (`KismetSystemLibrary.GetFrameCount`) (`self.CurrentFrame`))
    (`self.ApplyForce`)
    (else
      (`self.CleanForce`))))

(fn `ApplyForce`
  (`KismetSystemLibrary.PrintString` "Apply" true true (struct :`R` 1.0 :`B` 0.895627 :`A` 1.0) 0.05)
  (bind _returnvalue (`NiagaraFunctionLibrary.GetNiagaraParameterCollection` "/Game/TAcourse_III/Element/BaseElement/NPC_FxManager.NPC_FxManager"))
  (`NiagaraParameterCollectionInstance.SetBoolParameter` _returnvalue "ApplyForce?" true))

(fn `CleanForce`
  (`KismetSystemLibrary.PrintString` "Not Apply" true true (struct :`R` 0.273084 :`G` 1.0 :`A` 1.0) 0.05)
  (bind _returnvalue (`NiagaraFunctionLibrary.GetNiagaraParameterCollection` "/Game/TAcourse_III/Element/BaseElement/NPC_FxManager.NPC_FxManager"))
  (`NiagaraParameterCollectionInstance.SetBoolParameter` _returnvalue "ApplyForce?" false))

(fn `UserConstructionScript`)