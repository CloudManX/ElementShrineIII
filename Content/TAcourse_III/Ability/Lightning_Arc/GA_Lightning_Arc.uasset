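; Lightning Arc ability Blueprint that holds a main bolt effect active while its key is down.
; On key press, if the cooldown check returns false, it applies cooldown and spawns GE_Lightning_Arc_MainBolt at the ElementalPlayer's cursor location.
; Key release and cancel share one path that, guarded by the GameAbilityReleased flag, applies cooldown again and destroys the bolt.
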(event `self.CE_KeyPressed`
  (`parent.CE_KeyPressed`)
  (bind _cd (`self.CF_CdCheck`))
  (if (not _cd)
    (`self.CF_ApplyCd`)
    (set `self.bGameAbilityReleased` true)
    (bind _cursordata (`/Game/TAcourse_III/GameBP/Pawn/Player/B_ElementalPlayer.GetCursorData` (`self.ElementalPlayer`)))
    (bind _returnge (`self.SpawnGE` "/Game/TAcourse_III/Ability/Lightning_Arc/GE_Lightning_Arc_MainBolt.GE_Lightning_Arc_MainBolt_C" (`KismetMathLibrary.MakeTransform` (`.Location` (`GameplayStatics.BreakHitResult` _cursordata))) false true))
    (set `self.BoltGE` _returnge)))

(event `self.CE_KeyReleased`
  (if (`self.bGameAbilityReleased`) :!label _label
    (`self.CF_ApplyCd`)
    (set `self.bGameAbilityReleased` false)
    (`self.K2_DestroyActor` (`self.BoltGE`))))

(event `self.CE_Cancel`
  (goto _label))

(fn `UserConstructionScript`
  (`parent.UserConstructionScript`))