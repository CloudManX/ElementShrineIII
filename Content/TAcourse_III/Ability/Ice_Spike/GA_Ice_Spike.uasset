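; Ice Spike player ability that is aimed by holding and dragging the cursor, then spawns a line of ice spikes.
; Key press checks cooldown, anchors the start point and shows a box decal, which Tick orients toward the cursor over AttackRange.
; Release applies cooldown, hides the decal and spawns a staggered GE_Ice_Spike sequence along that fixed-length line.
; A near-zero drag falls back to a default direction.
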(event `self.CE_KeyPressed`
  ;[0.1483 1 0] CD Check
  (bind _cd (`self.CF_CdCheck`))
  (if (not _cd)
    (set `self.AbilityIsOn?` true)
    (set `self.CursorStartLocation` (`.Location` (`GameplayStatics.BreakHitResult` (`/Game/TAcourse_III/GameBP/Pawn/Player/B_ElementalPlayer.CursorData` (`self.ElementalPlayer`)))))
    (`SceneComponent.SetVisibility` (`self.UI_Box_Decal`) true false)))

(event `self.CE_KeyReleased`
  (bind _cursorstartlocation (`self.CursorStartLocation`))
  (bind _returnvalue (- (`self.CursorEndLocation`) _cursorstartlocation))
  ;[0.1483 1 0] CD Check
  (if (`self.AbilityIsOn?`)
    (`self.CF_ApplyCd`)
    (set `self.AbilityIsOn?` false)
    (set `self.CursorEndLocation` (`.Location` (`GameplayStatics.BreakHitResult` (`/Game/TAcourse_III/GameBP/Pawn/Player/B_ElementalPlayer.CursorData` (`self.ElementalPlayer`)))))
    (`SceneComponent.SetVisibility` (`self.UI_Box_Decal`) false false)
    (`/Game/TAcourse_III/GameBP/Combat/Macros_CombatBaseActor.SpawnGE_Sequence` "/Game/TAcourse_III/Ability/Ice_Spike/GE_Ice_Spike.GE_Ice_Spike_C" null 0.05 8 _cursorstartlocation (+ _cursorstartlocation (* (select `bool` (>= (`KismetMathLibrary.VSize` _returnvalue) 1.0) :`false` (1.0 0.0 0.0) :`true` (`KismetMathLibrary.Normal` _returnvalue)) (`self.AttackRange`))))))

(event `self.ReceiveTick`
  (params (DeltaSeconds :type "Float (single-precision)"))
  (bind _returnvalue (- (`self.CursorCurrentLocation`) (`self.CursorStartLocation`)))
  (bind _returnvalue_2 (>= (`KismetMathLibrary.VSize` _returnvalue) 1.0))
  (bind _output_get (set `self.CursorCurrentLocation` (`.Location` (`GameplayStatics.BreakHitResult` (`/Game/TAcourse_III/GameBP/Pawn/Player/B_ElementalPlayer.CursorData` (`self.ElementalPlayer`))))))
  (`SceneComponent.K2_SetWorldTransform` (`self.UI_Box_Decal`) (`KismetMathLibrary.MakeTransform` (+ (`self.CursorStartLocation`) (* (select `bool` _returnvalue_2 :`false` (1.0 0.0 0.0) :`true` (`KismetMathLibrary.Normal` _returnvalue)) (/ (`self.AttackRange`) 2.0))) (select `bool` _returnvalue_2 :`true` (`KismetMathLibrary.MakeRotator` (.roll (`KismetMathLibrary.FindLookAtRotation` (`self.CursorStartLocation`) _output_get)) (+ (.pitch (`KismetMathLibrary.FindLookAtRotation` (`self.CursorStartLocation`) _output_get)) -90.0) (.yaw (`KismetMathLibrary.FindLookAtRotation` (`self.CursorStartLocation`) _output_get)))) (`KismetMathLibrary.MakeVector` 100.0 100.0 (/ (`self.AttackRange`) 2.0))) false false))

(fn `UserConstructionScript`
  (`parent.UserConstructionScript`))