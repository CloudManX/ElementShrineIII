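; GA_Ice_Annihilate is the Ice Annihilate ability actor, cast when its key is released.
; On release it runs the cooldown check and, if that returns false, applies the cooldown and reads cursor data from ElementalPlayer.
; It then spawns GE_Ice_AnnihilateStartRing at the cursor location, passing UIMaxRadius as the ability radius and leaving any further effect to that actor.
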(event `self.CE_KeyReleased`
  ;[0 1 0] 默认情况下, 松开按键视为 cast 技能 并检查和设置CD
  (bind _cd (`self.CF_CdCheck`))
  (if (not _cd)
    (`self.CF_ApplyCd`)
    (bind _cursordata (`/Game/TAcourse_III/GameBP/Pawn/Player/B_ElementalPlayer.GetCursorData` (`self.ElementalPlayer`)))
    (`|SpawnActorFromClass` "/Game/TAcourse_III/Ability/Ice_Annihilate/GE_Ice_AnnihilateStartRing.GE_Ice_AnnihilateStartRing_C" (`KismetMathLibrary.MakeTransform` (`.Location` (`GameplayStatics.BreakHitResult` _cursordata))) "Undefined" "OverrideRootScale" null null (struct) (`self.UI_MaxRadius`) null)))

(fn `UserConstructionScript`
  (`parent.UserConstructionScript`))