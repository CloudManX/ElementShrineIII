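; GA_Fire_HellAttack is a fire ability that, on key release, pulls in meteor debris at the cursor and can ignite a storm there.
; The debris actor count sets the effect radius.
; Absorption briefly pulses a Niagara Parameter Collection with origin, radius and condition.
; With enough debris and the cooldown check passed, it also spawns the initial fire effect with that radius as a Niagara parameter.
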(event `self.CE_KeyReleased`
  (bind (_cursordata_bblockinghit _cursordata_binitialoverlap _cursordata_time _cursordata_distance _cursordata_location) (`GameplayStatics.BreakHitResult` (`/Game/TAcourse_III/GameBP/Pawn/Player/B_ElementalPlayer.CursorData` (`self.ElementalPlayer`))))
  ;[1 1 1] 默认情况下, 松开按键视为 cast 技能 并检查和设置CD
  (bind _cd (`self.CF_CdCheck`))
  (if (not _cd)
    (`self.CF_ApplyCd`)
    (set `self.Location` _cursordata_location)
    (bind _outactors (`GameplayStatics.GetAllActorsOfClass` "/Game/TAcourse_III/Ability/Fire_Meteor/GE_MeteorDebris.GE_MeteorDebris_C"))
    (bind _returnvalue (`KismetArrayLibrary.Array_Length` _outactors))
    (bind _output_get (set `self.Strom Radius` (`KismetMathLibrary.MapRangeClamped` (`KismetMathLibrary.Conv_IntToDouble` _returnvalue) 5.0 10.0 100.0 200.0)))
    (`self.CE_AbsorbEffect` (`self.Location`) _output_get)
    (if (>= _returnvalue (`self.MinNumberForIgnition`))
      (`self.CE_StormEffect` (`self.Location`) _output_get))))

(event `CE_AbsorbEffect`
  (params (Location :type "Vector Structure") (Radius :type "Float (double-precision)"))
  (bind _returnvalue (`NiagaraFunctionLibrary.GetNiagaraParameterCollection` "/Game/TAcourse_III/Ability/Fire_Hell_Attack/NPC_Hell_Attack.NPC_Hell_Attack"))
  (`NiagaraParameterCollectionInstance.SetFloatParameter` _returnvalue "Radius" Radius)
  (`NiagaraParameterCollectionInstance.SetVectorParameter` _returnvalue "Origin" Location)
  (`NiagaraParameterCollectionInstance.SetFloatParameter` _returnvalue "Condition" 1.0)
  (`KismetSystemLibrary.Delay` 0.2)
  (`NiagaraParameterCollectionInstance.SetFloatParameter` _returnvalue "Condition" 0.0))

(event `CE_StormEffect`
  (params (Center :type "Vector Structure") (Radius :type "Float (double-precision)"))
  (`KismetSystemLibrary.PrintString` "StormEffect" true true (struct :`R` 1.0 :`G` 0.310001 :`A` 1.0))
  ;[0 0.2108 1 1 14] 需要在GE中打开接受NiagaraParameter
  (`self.SpawnGE` "/Game/TAcourse_III/Ability/Fire_Hell_Attack/GE_Fire_Intial.GE_Fire_Intial_C" (`KismetMathLibrary.MakeTransform` Center) false false null 5.0 (make `/Game/TAcourse_III/GameBP/Combat/Struct_NiagaraParameter` Radius)))

(fn `UserConstructionScript`
  (`parent.UserConstructionScript`))