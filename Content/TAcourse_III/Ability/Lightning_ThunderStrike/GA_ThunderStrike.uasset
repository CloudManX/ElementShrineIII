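; GA_ThunderStrike is an actor-based lightning ability that casts a thunder bolt at the player's cursor.
; Releasing the key counts as the cast and runs a cooldown check, continuing only when that check returns false.
; It then applies the cooldown and spawns GE_ThunderBolt at the cursor location read from the ElementalPlayer's cursor data.
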(event `self.ReceiveBeginPlay`
  (`parent.ReceiveBeginPlay`))

(event `self.CE_KeyReleased`
  (bind (_cursordata_bblockinghit _cursordata_binitialoverlap _cursordata_time _cursordata_distance _cursordata_location) (`GameplayStatics.BreakHitResult` (`/Game/TAcourse_III/GameBP/Pawn/Player/B_ElementalPlayer.CursorData` (`self.ElementalPlayer`))))
  ;[1 1 1] 默认情况下, 松开按键视为 cast 技能 并检查和设置CD
  (bind _cd (`self.CF_CdCheck`))
  (if (not _cd)
    (`self.CF_ApplyCd`)
    (bind _output_get (set `self.Location` _cursordata_location))
    (`self.SpawnGE` "/Game/TAcourse_III/Ability/Lightning_ThunderStrike/GE_ThunderBolt.GE_ThunderBolt_C" (`KismetMathLibrary.MakeTransform` _output_get))))

(fn `UserConstructionScript`
  (`parent.UserConstructionScript`))